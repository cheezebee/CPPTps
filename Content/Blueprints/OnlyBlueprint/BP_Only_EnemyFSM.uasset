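; Enemy AI state machine component that drives its owning BP_Only_Enemy against the player through Idle, Move, Attack, AttackDelay, Damaged and Die.
; A 60-degree view cone plus line trace selects chasing or random NavMesh wandering via AIController.
; ChangeState mirrors state to the AnimBP and plays damage or death montages; attacks only print text.
; Dead enemies sink once DieMove is set, then reset and return to the EnemyManager's pool.
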(event `self.ReceiveBeginPlay`
  ;[1 1 1] Target 찾자 (Player)
  (bind _returnvalue (`GameplayStatics.GetActorOfClass` "/Game/Blueprints/OnlyBlueprint/BP_Only_TpsPlayer.BP_Only_TpsPlayer_C"))
  (set `self.target` _returnvalue)
  ;[1 1 1] 나를 찾자
  (bind _asbp_only_enemy (cast `/Game/Blueprints/OnlyBlueprint/BP_Only_Enemy` (`self.GetOwner`)))
  (set `self.me` _asbp_only_enemy)
  ;[1 1 1] 초기 HP 설정
  (set `self.currHP` (`self.maxHP`))
  (bind _asabp_only_enemy (cast `/Game/Blueprints/OnlyBlueprint/ABP_Only_Enemy` (`SkeletalMeshComponent.GetAnimInstance` (`Character.Mesh` (`self.me`)))))
  (set `self.anim` _asabp_only_enemy)
  (bind _asaicontroller (cast `AIController` (`Pawn.GetController` (`self.me`))))
  (set `self.ai` _asaicontroller))

(event `self.ReceiveTick`
  (params (DeltaSeconds :type "Float (single-precision)"))
  (switch `/Game/Blueprints/OnlyBlueprint/BP_EnemyState` (`self.state`)
    (:`NewEnumerator0`
      (`self.UpdateIdle`))
    (:`NewEnumerator1`
      (`self.Update Move`))
    (:`NewEnumerator2`
      (`self.UpdateAttack`))
    (:`NewEnumerator3`
      (`self.UpdateDamaged`))
    (:`NewEnumerator4`
      (`self.UpdateDie`))
    (:`NewEnumerator5`
      (`self.UpdateAttackDelay`))))

(fn `Change State`
  (params (s :type "/Game/Blueprints/OnlyBlueprint/BP_EnemyState Enum" :default "NewEnumerator0"))
  (`Controller.StopMovement` (`self.ai`))
  (bind _output_get (set `self.state` s))
  (bind _output_get_2 (set `/Game/Blueprints/OnlyBlueprint/ABP_Only_Enemy.state` _output_get (`self.anim`)))
  (switch `/Game/Blueprints/OnlyBlueprint/BP_EnemyState` _output_get_2
    (:`NewEnumerator1`
      (bind _output_get_3 (set `self.randPos` (`NavigationSystemV1.K2_GetRandomReachablePointInRadius` (`NavigationSystemV1.GetNavigationSystem`) (`Actor.K2_GetActorLocation` (`self.me`)) 500.0 null null)))
      (`KismetSystemLibrary.PrintString` (`KismetStringLibrary.Conv_VectorToString` _output_get_3)))
    (:`NewEnumerator3`
      (`Character.PlayAnimMontage` (`self.me`) "/Game/Blueprints/AMT_EnemyDamaged.AMT_EnemyDamaged" 1.0 (`KismetStringLibrary.Conv_StringToName` (`KismetStringLibrary.Concat_StrStr` "Damage" (`KismetStringLibrary.Conv_IntToString` (`KismetMathLibrary.RandomIntegerInRange` 0 1))))))
    (:`NewEnumerator4`
      (`PrimitiveComponent.SetCollisionEnabled` (`Character.CapsuleComponent` (`self.me`)) "NoCollision")
      (`Character.PlayAnimMontage` (`self.me`) "/Game/Blueprints/AMT_EnemyDamaged.AMT_EnemyDamaged" 1.0 "Die"))))

(fn `Is Target Trace`
  (returns (bTrace :type Boolean))
  (bind _returnvalue (< (`KismetMathLibrary.DegAcos` (`KismetMathLibrary.Dot_VectorVector` (`Actor.GetActorForwardVector` (`self.me`)) (`KismetMathLibrary.Normal` (- (`Actor.K2_GetActorLocation` (`self.target`)) (`Actor.K2_GetActorLocation` (`self.me`)))))) 30.0))
  ;[1 1 1] 만약에 두 벡터 사이의 각이 30보다 작으면 (시야60) Move 상태로 한다.
  (if _returnvalue
    (bind _outhit (`KismetSystemLibrary.LineTraceSingle` (`Actor.K2_GetActorLocation` (`self.me`)) (`Actor.K2_GetActorLocation` (`self.target`)) "TraceTypeQuery1"))
    (return (and _returnvalue (`KismetStringLibrary.Contains` (`KismetSystemLibrary.GetDisplayName` (`.HitActor` (`GameplayStatics.BreakHitResult` _outhit))) "Player")))))

(fn `IsWaitComplete`
  (params (delayTime :type "Float (double-precision)"))
  (returns (bComplete :type Boolean))
  (bind _output_get (set `self.currTime` (+ (`self.currTime`) (`GameplayStatics.GetWorldDeltaSeconds`))))
  (if (== (> _output_get delayTime) true)
    (set `self.currTime` 0.0)
    (return true)
    (else
      (return false))))

(fn `ReceiveDamage`
  ;[1 1 1] currHP--;
  (bind _output_get (set `self.currHP` (- (`self.currHP`) 1.0)))
  ;[1 1 1] if(currHP > 0) { 피격상태 } else { 죽음상태 }
  (if (> _output_get 0.0)
    (`self.Change State` "NewEnumerator3")
    (else
      (`self.Change State` "NewEnumerator4"))))

(fn `Update Move`
  (bind _returnvalue (`Actor.K2_GetActorLocation` (`self.target`)))
  (bind _btrace (`self.Is Target Trace`))
  (if _btrace
    ;[1 1 1] 만약에 공격범위에 target 이 들어왔다면 상태를 Attack 으로!
    (if (< (`KismetMathLibrary.VSize` (- _returnvalue (`Actor.K2_GetActorLocation` (`self.me`)))) (`self.attackRange`))
      (`self.Change State` "NewEnumerator2")
      (else
        (`AIController.MoveToLocation` (`self.ai`) _returnvalue -1.0 true true false true null true)))
    (else
      (bind _returnvalue_2 (`AIController.MoveToLocation` (`self.ai`) (`self.randPos`) -1.0 true true false true null true))
      (if (`|EnumEquality` _returnvalue_2 "AlreadyAtGoal")
        (`self.Change State` "NewEnumerator0")))))

(fn `UpdateAttack`
  (`KismetSystemLibrary.PrintString` "Attack!!!!!!")
  (`self.Change State` "NewEnumerator5"))

(fn `UpdateAttackDelay`
  (bind _bcomplete (`self.IsWaitComplete` (`self.attackDelayTime`)))
  (if _bcomplete
    ;[1 1 1] 만약에 target 과 me 의 거리가 attackRange 보다 작으면 공격!! 출력, 그렇지 않으면 Idle 상태로 전환
    (if (< (`KismetMathLibrary.VSize` (- (`Actor.K2_GetActorLocation` (`self.target`)) (`Actor.K2_GetActorLocation` (`self.me`)))) (`self.attackRange`))
      (`self.Change State` "NewEnumerator2")
      (else
        (`self.Change State` "NewEnumerator0")))))

(fn `UpdateDamaged`
  (bind _bcomplete (`self.IsWaitComplete` (`self.damageDelayTime`)))
  (if _bcomplete
    (`self.Change State` "NewEnumerator0")))

(fn `UpdateDie`
  (bind _me (`self.me`))
  (bind (_returnvalue_x _returnvalue_y _returnvalue_z) (`KismetMathLibrary.BreakVector` (`Actor.K2_GetActorLocation` (`self.me`))))
  (if (`self.bDieMove`)
    (`Actor.K2_SetActorLocation` (`self.me`) (+ (`Actor.K2_GetActorLocation` (`self.me`)) (* (* (`KismetMathLibrary.Vector_Down`) (`self.dieSpeed`)) (`GameplayStatics.GetWorldDeltaSeconds`))) false false)
    ;[1 1 1] if(me.location.Z < -200) ...
    (if (< _returnvalue_z -200.0)
      (`self.Change State` "NewEnumerator0")
      (set `self.currHP` (`self.maxHP`))
      (set `self.bDieMove` false)
      (`Character.StopAnimMontage` _me "/Game/Blueprints/AMT_EnemyDamaged.AMT_EnemyDamaged")
      (`/Game/Blueprints/OnlyBlueprint/BP_Only_Enemy.Set Active` _me false)
      (bind _returnvalue (`GameplayStatics.GetActorOfClass` "/Game/Blueprints/OnlyBlueprint/BP_Only_EnemyManager.BP_Only_EnemyManager_C"))
      (`KismetArrayLibrary.Array_Add` (`/Game/Blueprints/OnlyBlueprint/BP_Only_EnemyManager.enemyArray` _returnvalue) (`self.me`)))))

(fn `UpdateIdle`
  (bind _btrace (`self.Is Target Trace`))
  (if _btrace
    (`self.Change State` "NewEnumerator1")
    (else
      (bind _bcomplete (`self.IsWaitComplete` (`self.IdleDelayTime`)))
      (if _bcomplete
        (`self.Change State` "NewEnumerator1")))))