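; BP_Only_EnemyManager is an object-pooled spawner that releases BP_Only_Enemy actors at its own location at random intervals.
; BeginPlay pre-spawns a small set of enemies, deactivates them and stores them in EnemyArray.
; While the pool has entries, Tick runs a timer that activates the first enemy, moves it to the manager, removes it from the array and re-rolls the delay.
; AddEnemy appends an enemy to the pool.
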(event `self.ReceiveBeginPlay`
  (set `self.createTime` (`KismetMathLibrary.RandomFloatInRange` 1.0 5.0))
  (for _ (range 2)
    (bind _returnvalue (`|SpawnActorFromClass` "/Game/Blueprints/OnlyBlueprint/BP_Only_Enemy.BP_Only_Enemy_C" (`self.GetTransform`) "Undefined" "OverrideRootScale" null null))
    (`KismetArrayLibrary.Array_Add` (`self.enemyArray`) _returnvalue)
    (`/Game/Blueprints/OnlyBlueprint/BP_Only_Enemy.Set Active` _returnvalue false)))

(event `self.ReceiveTick`
  (params (DeltaSeconds :type "Float (single-precision)"))
  (bind _enemyarray (`self.enemyArray`))
  (bind _output (`|GetArrayItem` _enemyarray))
  (if (> (`KismetArrayLibrary.Array_Length` (`self.enemyArray`)) 0)
    (bind _output_get (set `self.currTime` (+ DeltaSeconds (`self.currTime`))))
    (if (> _output_get (`self.createTime`))
      (set `self.createTime` (`KismetMathLibrary.RandomFloatInRange` 1.0 5.0))
      (set `self.currTime` 0.0)
      (`/Game/Blueprints/OnlyBlueprint/BP_Only_Enemy.Set Active` _output true)
      (`self.K2_SetActorLocation` _output (`self.K2_GetActorLocation`) false false)
      (`KismetArrayLibrary.Array_Remove` _enemyarray))))

(fn `AddEnemy`
  (params (e :type "/Game/Blueprints/OnlyBlueprint/BP_Only_Enemy Object Reference"))
  (`KismetArrayLibrary.Array_Add` (`self.enemyArray`) e))

(fn `UserConstructionScript`)