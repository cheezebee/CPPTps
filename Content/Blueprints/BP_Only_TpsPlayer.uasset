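; BP_Only_TpsPlayer is a Blueprint-only third-person player with WASD movement and mouse-style camera look.
; Axis inputs store move directions and accumulate turn and look values, which Tick applies through MoveAction and RotateAction.
; Movement sets location directly along normalized actor forward and right vectors at WalkSpeed, without sweeping.
; Controller rotation is disabled: accumulated yaw turns the actor, while inverted, unclamped pitch tilts the SpringArm.
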(event `self.ReceiveBeginPlay`
  (set `self.bUseControllerRotationYaw` false)
  (set `SpringArmComponent.bUsePawnControlRotation` false (`self.SpringArm`)))

(event `self.ReceiveTick`
  (params (DeltaSeconds :type "Float (single-precision)"))
  (`self.Move Action` DeltaSeconds)
  (`self.RotateAction`))

(event `InputAxis|Horizontal`
  (params (AxisValue :type "Float (single-precision)"))
  ;[1 1 1] W, A, S, D
  (set `self.dirH` AxisValue))

(event `InputAxis|Vertical`
  (params (AxisValue :type "Float (single-precision)"))
  ;[1 1 1] W, A, S, D
  (set `self.dirV` AxisValue))

(event `InputAxis|Turn`
  (params (AxisValue :type "Float (single-precision)"))
  ;[1 1 1] 카메라 회전
  (set `self.mx` (+ AxisValue (`self.mx`))))

(event `InputAxis|LookUp`
  (params (AxisValue :type "Float (single-precision)"))
  ;[1 1 1] 카메라 회전
  (set `self.my` (+ AxisValue (`self.my`))))

(fn `Move Action`
  (params (deltaTime :type "Float (double-precision)"))
  (`self.K2_SetActorLocation` (+ (`self.K2_GetActorLocation`) (* deltaTime (* (`KismetMathLibrary.Normal` (+ (* (`self.dirV`) (`self.GetActorForwardVector`)) (* (`self.dirH`) (`self.GetActorRightVector`)))) (`self.walkSpeed`))))))

(fn `RotateAction`
  (`self.K2_SetActorRotation` (`KismetMathLibrary.MakeRotator` 0.0 0.0 (`self.mx`)))
  (`SceneComponent.K2_SetRelativeRotation` (`self.SpringArm`) (`KismetMathLibrary.MakeRotator` 0.0 (* (`self.my`) -1.0)) false false))

(fn `UserConstructionScript`)